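; AI-driven ant enemy that wanders, chases the 2D player character on sight, and damages it on contact.
; While no player is seen, Tick moves it after random delays to reachable points, keeping only their X so it roams along one axis.
; PawnSensing starts the chase and sets CanSeeEnemy, which a retriggerable delay clears shortly after sightings stop.
; Box overlap with the player applies fixed damage.
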(event OnSeePawn(PawnSensing)
  (params (Pawn :type Pawn%20Object%20Reference))
  (bind _as2dplayer_character (Utilities|Casting|CastTo2DPlayerCharacter Pawn))
  (Utilities|FlowControl|Sequence
    (:then_0
      (Variables|Default|SetCanSeeEnemy true)
      (AI|AIMoveTo self "0, 0, 0" _as2dplayer_character 5.0 false))
    (:then_1
      (Utilities|FlowControl|RetriggerableDelay 0.5)
      (Variables|Default|SetCanSeeEnemy false))))

(event OnComponentBeginOverlap(Box)
  (params (OverlappedComponent :type Primitive%20Component%20Object%20Reference) (OtherActor :type Actor%20Object%20Reference) (OtherComp :type Primitive%20Component%20Object%20Reference) (OtherBodyIndex :type Integer) (bFromSweep :type Boolean) (SweepResult :type Hit%20Result%20Structure%20%28by%20ref%29))
  (bind _as2dplayer_character (Utilities|Casting|CastTo2DPlayerCharacter OtherActor))
  (Game|Damage|ApplyDamage _as2dplayer_character 1e+01 0 0))

(event EventBeginPlay)

(event Collision|EventActorBeginOverlap
  (params (OtherActor :type Actor%20Object%20Reference)))

(event EventTick
  (params (DeltaSeconds :type Float%20%28single-precision%29))
  (bind _returnvalue (Transformation|GetActorLocation))
  (bind (_x _y _z) (Class|KismetMathLibrary|BreakVector3f _returnvalue))
  (if (not (Variables|Default|GetCanSeeEnemy))
    (Utilities|FlowControl|Delay (Math|Random|RandomFloatinRange 2.0 5.0))
    (AI|AIMoveTo self (Math|Vector|MakeVector (.X (Class|KismetMathLibrary|BreakVector3f (.RandomLocation (AI|Navigation|GetRandomReachablePointinRadius _returnvalue 1e+03 0 0)))) _y _z) 0 5.0 false)))

(fn ConstructionScript)